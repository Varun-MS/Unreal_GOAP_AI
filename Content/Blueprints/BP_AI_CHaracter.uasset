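; AI combatant character driven by GOAP, pursuing goals to find enemies, weapons, kill or preserve itself.
; The construction script builds world-state definers, goals, and actions with preconditions and effects.
; A looping timer asks the goal manager for a goal, sending a new plan to the action manager when it changes.
; Tick refreshes world state and billboarded debug text, while overlaps grant pickups and a shield absorbs one hit.
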(event `self.ReceiveBeginPlay`
  (`self.SpawnDefaultController`)
  (`|ExecutionSequence`
    (:`then_0`
      ;[1 1 1] Setting Up references and dependencies
      (bind _asbp_aicontroller_goap (cast `/Game/Blueprints/BP_AIController_Goap` (`self.GetController`)))
      (bind _output_get (set `self.ControllerRef` _asbp_aicontroller_goap))
      (`ActionManager.SetAIController` (`self.BP_AC_ActionManager`) _output_get)
      (`ActionManager.SetWorldStateManager` (`self.BP_AC_ActionManager`) (`self.BP_AC_WorldStateManager`))
      (for (_array_element _array_index) (`self.AllActions`)
        (`ActionTest.SetActionID` _array_element _array_index)))
    (:`then_1`
      ;[1 1 1] Check Every 3 Seconds to Ensure the Current Goal is Still Viable. If the current goal is unviable, a new goal is returned. With this new goal in mind, generate a new plan, and send it to the Action Manager
      (`KismetSystemLibrary.K2_SetTimerDelegate` (delegate `Ensure Goal Viability`) 3.0 true))))

(event `Ensure Goal Viability`
  ;[1 1 1] Check Every 3 Seconds to Ensure the Current Goal is Still Viable. If the current goal is unviable, a new goal is returned. With this new goal in mind, generate a new plan, and send it to the Action Manager
  (if (`self.IsAlive`)
    (set `self.PreviousGoal` (`self.CurrentGoal`))
    (bind _output_get (set `self.CurrentGoal` (`GoalManager.GetNewGoal` (`self.BP_AC_GoalManager`) (`self.BP_AC_WorldStateManager`))))
    (if (!= _output_get (`self.PreviousGoal`))
      (bind _returnvalue (`ActionPlanner.Plan` (`self.BP_AC_ActionPlanner`) (`WorldStateManager.CurrentWorldState` (`self.BP_AC_WorldStateManager`)) (`self.CurrentGoal`) (`self.AllActions`)))
      (`ActionManager.SchedulePlan` (`self.BP_AC_ActionManager`) _returnvalue))
    (else
      (`ActionManager.ClearCurrentPlan` (`self.BP_AC_ActionManager`)))))

(event `self.ReceiveTick`
  (params (DeltaSeconds :type "Float (single-precision)"))
  (bind _currentgoal (`self.CurrentGoal`))
  (bind _currentworldstate (`WorldStateManager.CurrentWorldState` (`self.BP_AC_WorldStateManager`)))
  (if (`self.IsAlive`)
    ;[1 1 1] Billboard Debug Text
    (`SceneComponent.K2_SetWorldRotation` (`self.Goal_Status`) (`KismetMathLibrary.FindLookAtRotation` (`self.K2_GetActorLocation`) (`self.K2_GetActorLocation` (`GameplayStatics.GetPlayerCharacter` 0))) false false)
    ;[1 1 1] Billboard Debug Text
    (`SceneComponent.K2_SetWorldRotation` (`self.CurrentAction_Status`) (`KismetMathLibrary.FindLookAtRotation` (`self.K2_GetActorLocation`) (`self.K2_GetActorLocation` (`GameplayStatics.GetPlayerCharacter` 0))) false false)
    ;[1 1 1] Billboard Debug Text
    (`SceneComponent.K2_SetWorldRotation` (`self.HasLowHealth_Status`) (`KismetMathLibrary.FindLookAtRotation` (`self.K2_GetActorLocation`) (`self.K2_GetActorLocation` (`GameplayStatics.GetPlayerCharacter` 0))) false false)
    ;[1 1 1] Billboard Debug Text
    (`SceneComponent.K2_SetWorldRotation` (`self.HasShield_Status`) (`KismetMathLibrary.FindLookAtRotation` (`self.K2_GetActorLocation`) (`self.K2_GetActorLocation` (`GameplayStatics.GetPlayerCharacter` 0))) false false)
    ;[1 1 1] Billboard Debug Text
    (`SceneComponent.K2_SetWorldRotation` (`self.IsEnemyVisible_Status`) (`KismetMathLibrary.FindLookAtRotation` (`self.K2_GetActorLocation`) (`self.K2_GetActorLocation` (`GameplayStatics.GetPlayerCharacter` 0))) false false)
    ;[1 1 1] Billboard Debug Text
    (`SceneComponent.K2_SetWorldRotation` (`self.HasWeapon_Status`) (`KismetMathLibrary.FindLookAtRotation` (`self.K2_GetActorLocation`) (`self.K2_GetActorLocation` (`GameplayStatics.GetPlayerCharacter` 0))) false false)
    ;[1 1 1] Billboard Debug Text
    (`SceneComponent.K2_SetWorldRotation` (`self.IsEnemyDead_Status`) (`KismetMathLibrary.FindLookAtRotation` (`self.K2_GetActorLocation`) (`self.K2_GetActorLocation` (`GameplayStatics.GetPlayerCharacter` 0))) false false)
    ;[1 1 1] Recalculate World State to Ensure it is Constantly Up to Date
    (`WorldStateManager.RecalculateWorldState` (`self.BP_AC_WorldStateManager`) self)
    (`|ExecutionSequence`
      (:`then_0`
        (bind _returnvalue (`WorldState.GetWorldStateDefiner` _currentworldstate (enumliteral `/Game/Blueprints/EWorldState` "NewEnumerator0")))
        (`TextRenderComponent.K2_SetText` (`self.HasLowHealth_Status`) (`KismetTextLibrary.Conv_StringToText` (`KismetStringLibrary.Concat_StrStr` "HasLowHealth: " (`KismetStringLibrary.Conv_BoolToString` (`WorldStateDefiner.IsTrue` _returnvalue))))))
      (:`then_1`
        (bind _returnvalue_2 (`WorldState.GetWorldStateDefiner` _currentworldstate (enumliteral `/Game/Blueprints/EWorldState` "NewEnumerator1")))
        (`TextRenderComponent.K2_SetText` (`self.HasWeapon_Status`) (`KismetTextLibrary.Conv_StringToText` (`KismetStringLibrary.Concat_StrStr` "HasWeapon: " (`KismetStringLibrary.Conv_BoolToString` (`WorldStateDefiner.IsTrue` _returnvalue_2))))))
      (:`then_2`
        (bind _returnvalue_3 (`WorldState.GetWorldStateDefiner` _currentworldstate (enumliteral `/Game/Blueprints/EWorldState` "NewEnumerator2")))
        (`TextRenderComponent.K2_SetText` (`self.HasShield_Status`) (`KismetTextLibrary.Conv_StringToText` (`KismetStringLibrary.Concat_StrStr` "HasShield: " (`KismetStringLibrary.Conv_BoolToString` (`WorldStateDefiner.IsTrue` _returnvalue_3))))))
      (:`then_3`
        (bind _returnvalue_4 (`WorldState.GetWorldStateDefiner` _currentworldstate (enumliteral `/Game/Blueprints/EWorldState` "NewEnumerator3")))
        (`TextRenderComponent.K2_SetText` (`self.IsEnemyVisible_Status`) (`KismetTextLibrary.Conv_StringToText` (`KismetStringLibrary.Concat_StrStr` "IsEnemyVisible: " (`KismetStringLibrary.Conv_BoolToString` (`WorldStateDefiner.IsTrue` _returnvalue_4))))))
      (:`then_4`
        (bind _returnvalue_5 (`WorldState.GetWorldStateDefiner` _currentworldstate (enumliteral `/Game/Blueprints/EWorldState` "NewEnumerator4")))
        (`TextRenderComponent.K2_SetText` (`self.IsEnemyDead_Status`) (`KismetTextLibrary.Conv_StringToText` (`KismetStringLibrary.Concat_StrStr` "IsEnemyDead: " (`KismetStringLibrary.Conv_BoolToString` (`WorldStateDefiner.IsTrue` _returnvalue_5))))))
      (:`then_5`
        (`/Engine/EditorBlueprintResources/StandardMacros.IsValid` _currentgoal
          (:`Is Valid`
            (`TextRenderComponent.K2_SetText` (`self.Goal_Status`) (`KismetTextLibrary.Conv_StringToText` (`WorldState.HumanReadableName` _currentgoal)))))))))

(event `self.CapsuleComponent.OnComponentBeginOverlap`
  (params (OverlappedComponent :type "PrimitiveComponent Object Reference") (OtherActor :type "Actor Object Reference") (OtherComp :type "PrimitiveComponent Object Reference") (OtherBodyIndex :type Integer) (bFromSweep :type Boolean) (SweepResult :type "HitResult Structure (by ref)"))
  ;[1 1 1] Handle Pickups
  (bind _pickuptype (message `/Game/Blueprints/BP_I_Pickup.GetPickupType` OtherActor))
  (switch `/Game/Blueprints/EPickupType` _pickuptype
    (:`NewEnumerator0`
      (`self.Heal` 50.0))
    (:`NewEnumerator1`
      (set `self.HasShield` true))
    (:`NewEnumerator2`
      (set `self.HasWeapon` true))))

(fn `CheckIfEnemyIsVisible`
  (returns (IsVisible :type Boolean))
  (bind _outhit (`KismetSystemLibrary.LineTraceSingle` :`Start` (`self.K2_GetActorLocation`) :`End` (`self.K2_GetActorLocation` (`self.EnemyRef`)) :`TraceChannel` "TraceTypeQuery2" :`DrawDebugType` "ForOneFrame"))
  (return (== (`.HitActor` (`GameplayStatics.BreakHitResult` _outhit)) (`self.EnemyRef`))))

(fn `DoDamage`
  (params (DamageAmount :type "Float (double-precision)"))
  (if (`self.HasShield`)
    (set `self.HasShield` false)
    (else
      (bind _output_get (set `self.Health` (- (`self.Health`) DamageAmount)))
      (if (<= _output_get 40.0)
        (if (<= _output_get 0.0)
          (set `self.IsAlive` false)
          (`KismetSystemLibrary.PrintString` "I DIED!"))
        (else
          (`KismetSystemLibrary.PrintString` "TOOK DAMAGE!"))))))

(fn `Heal`
  (params (HealAmount :type "Float (double-precision)"))
  (bind _health (`self.Health`))
  (bind _returnvalue (+ _health HealAmount))
  (if (> _returnvalue _health)
    (set `self.Health` 100.0)
    (else
      (set `self.Health` _returnvalue))))

(fn `SetStatus`
  (params (NewParam :type String))
  (bind _output_get (set `self.CurrentAction_DebugStatus` (`KismetTextLibrary.Conv_StringToText` NewParam)))
  (`TextRenderComponent.K2_SetText` (`self.CurrentAction_Status`) _output_get))

(fn `UserConstructionScript`
  (bind _returnvalue (enumliteral `/Game/Blueprints/EWorldState` "NewEnumerator1"))
  (bind _returnvalue_2 (enumliteral `/Game/Blueprints/EWorldState` "NewEnumerator4"))
  (bind _returnvalue_3 (enumliteral `/Game/Blueprints/EWorldState` "NewEnumerator2"))
  (bind _returnvalue_4 (enumliteral `/Game/Blueprints/EWorldState` "NewEnumerator0"))
  (bind _findenemyaction (`self.FindEnemyAction`))
  (bind _findenemy_goal (`self.FindEnemy_Goal`))
  (bind _bp_ac_worldstatemanager (`self.BP_AC_WorldStateManager`))
  (bind _bp_ac_goalmanager (`self.BP_AC_GoalManager`))
  (bind _killenemy_goal (`self.KillEnemy_Goal`))
  (bind _preserveself_goal (`self.PreserveSelf_Goal`))
  (bind _findhealthaction (`self.FindHealthAction`))
  (bind _findweaponaction (`self.FindWeaponAction`))
  (bind _meleeaction (`self.MeleeAction`))
  (bind _shootaction (`self.ShootAction`))
  (bind _shieldaction (`self.ShieldAction`))
  (bind _findweapon_goal (`self.FindWeapon_Goal`))
  (bind _currentworldstate (`WorldStateManager.CurrentWorldState` (`self.BP_AC_WorldStateManager`)))
  ;[1 1 1] Construct Current World State
  (bind _returnvalue_5 (`|GenericCreateObject` "/Script/FPSGame.WorldState" (`self.BP_AC_WorldStateManager`)))
  (`WorldStateManager.InitializeCurrentWorldState` (`self.BP_AC_WorldStateManager`) _returnvalue_5)
  ;[1 1 1] Construct World State Definers
  (`|ExecutionSequence`
    (:`then_0`
      (bind _returnvalue_6 (`|GenericCreateObject` "/Game/Blueprints/GOAP/WorldStateDefiners/HasLowHealth.HasLowHealth_C" _bp_ac_worldstatemanager))
      (set `self.HasLowHealthDefiner` _returnvalue_6))
    (:`then_1`
      (bind _returnvalue_7 (`|GenericCreateObject` "/Game/Blueprints/GOAP/WorldStateDefiners/HasShield.HasShield_C" _bp_ac_worldstatemanager))
      (set `self.HasShieldDefiner` _returnvalue_7))
    (:`then_2`
      (bind _returnvalue_8 (`|GenericCreateObject` "/Game/Blueprints/GOAP/WorldStateDefiners/HasWeapon.HasWeapon_C" _bp_ac_worldstatemanager))
      (set `self.HasWeaponDefiner` _returnvalue_8))
    (:`then_3`
      (bind _returnvalue_9 (`|GenericCreateObject` "/Game/Blueprints/GOAP/WorldStateDefiners/IsEnemyDead.IsEnemyDead_C" _bp_ac_worldstatemanager))
      (set `self.IsEnemyDeadDefiner` _returnvalue_9))
    (:`then_4`
      (bind _returnvalue_10 (`|GenericCreateObject` "/Game/Blueprints/GOAP/WorldStateDefiners/IsEnemyVisible.IsEnemyVisible_C" _bp_ac_worldstatemanager))
      (set `self.IsEnemyVisibleDefiner` _returnvalue_10)
      ;[1 1 1] Construct Actions
      (`|ExecutionSequence`
        (:`then_0`
          (bind _returnvalue_11 (`|GenericCreateObject` "/Game/Blueprints/GOAP/Actions/BP_Action_FindEnemy.BP_Action_FindEnemy_C" self))
          (set `self.FindEnemyAction` _returnvalue_11))
        (:`then_1`
          (bind _returnvalue_12 (`|GenericCreateObject` "/Game/Blueprints/GOAP/Actions/BP_Action_FindHealth.BP_Action_FindHealth_C" self))
          (set `self.FindHealthAction` _returnvalue_12))
        (:`then_2`
          (bind _returnvalue_13 (`|GenericCreateObject` "/Game/Blueprints/GOAP/Actions/BP_Action_FindWeapon.BP_Action_FindWeapon_C" self))
          (set `self.FindWeaponAction` _returnvalue_13))
        (:`then_3`
          (bind _returnvalue_14 (`|GenericCreateObject` "/Game/Blueprints/GOAP/Actions/BP_Action_Melee.BP_Action_Melee_C" self))
          (set `self.MeleeAction` _returnvalue_14))
        (:`then_4`
          (bind _returnvalue_15 (`|GenericCreateObject` "/Game/Blueprints/GOAP/Actions/BP_Action_Shoot.BP_Action_Shoot_C" self))
          (set `self.ShootAction` _returnvalue_15))
        (:`then_5`
          (bind _returnvalue_16 (`|GenericCreateObject` "/Game/Blueprints/GOAP/Actions/BP_Action_FindShield.BP_Action_FindShield_C" self))
          (set `self.ShieldAction` _returnvalue_16)
          ;[1 1 1] Construct Goals and add them to the Goal Manager
          (`|ExecutionSequence`
            (:`then_0`
              (bind _returnvalue_17 (`|GenericCreateObject` "/Game/Blueprints/GOAP/Goals/FindWeapon.FindWeapon_C" self))
              (set `self.FindWeapon_Goal` _returnvalue_17))
            (:`then_1`
              (bind _returnvalue_18 (`|GenericCreateObject` "/Game/Blueprints/GOAP/Goals/FindEnemy.FindEnemy_C" self))
              (set `self.FindEnemy_Goal` _returnvalue_18))
            (:`then_2`
              (bind _returnvalue_19 (`|GenericCreateObject` "/Game/Blueprints/GOAP/Goals/KillEnemy.KillEnemy_C" self))
              (set `self.KillEnemy_Goal` _returnvalue_19))
            (:`then_3`
              (bind _returnvalue_20 (`|GenericCreateObject` "/Game/Blueprints/GOAP/Goals/PreserveSelf.PreserveSelf_C" self))
              (set `self.PreserveSelf_Goal` _returnvalue_20)
              (`|ExecutionSequence`
                (:`then_0`
                  (bind _returnvalue_21 (`|GenericCreateObject` "/Game/Blueprints/GOAP/WorldStateDefiners/IsEnemyVisible.IsEnemyVisible_C" self))
                  (set `WorldStateDefiner.IsTrue` true _returnvalue_21)
                  (`WorldState.AddWorldStateDefiner` _findenemy_goal (enumliteral `/Game/Blueprints/EWorldState` "NewEnumerator3") _returnvalue_21)
                  (set `WorldState.HumanReadableName` "Find Enemy" _findenemy_goal)
                  (`GoalManager.AddGoal` _bp_ac_goalmanager (`self.FindEnemy_Goal`)))
                (:`then_1`
                  (bind _returnvalue_22 (`|GenericCreateObject` "/Game/Blueprints/GOAP/WorldStateDefiners/HasLowHealth.HasLowHealth_C" self))
                  (`WorldState.AddWorldStateDefiner` _preserveself_goal (enumliteral `/Game/Blueprints/EWorldState` "NewEnumerator0") _returnvalue_22)
                  (set `WorldState.HumanReadableName` "Preserve Self" _preserveself_goal)
                  (`GoalManager.AddGoal` _bp_ac_goalmanager (`self.PreserveSelf_Goal`)))
                (:`then_2`
                  (bind _returnvalue_23 (`|GenericCreateObject` "/Game/Blueprints/GOAP/WorldStateDefiners/IsEnemyDead.IsEnemyDead_C" self))
                  (set `WorldStateDefiner.IsTrue` true _returnvalue_23)
                  (`WorldState.AddWorldStateDefiner` _killenemy_goal (enumliteral `/Game/Blueprints/EWorldState` "NewEnumerator4") _returnvalue_23)
                  (set `WorldState.HumanReadableName` "Kill Enemy" _killenemy_goal)
                  (`GoalManager.AddGoal` _bp_ac_goalmanager (`self.KillEnemy_Goal`)))
                (:`then_3`
                  (bind _returnvalue_24 (`|GenericCreateObject` "/Game/Blueprints/GOAP/WorldStateDefiners/HasWeapon.HasWeapon_C" self))
                  (set `WorldStateDefiner.IsTrue` true _returnvalue_24)
                  (`WorldState.AddWorldStateDefiner` _findweapon_goal (enumliteral `/Game/Blueprints/EWorldState` "NewEnumerator1") _returnvalue_24)
                  (set `WorldState.HumanReadableName` "Find Weapon" _findweapon_goal)
                  (`GoalManager.AddGoal` _bp_ac_goalmanager (`self.FindWeapon_Goal`))
                  ;[1 1 1] Setting Up the Current World State
                  (`|ExecutionSequence`
                    (:`then_0`
                      ;;[1 1 1] Has Low Health
                      (`WorldState.AddWorldStateDefiner` _currentworldstate (enumliteral `/Game/Blueprints/EWorldState` "NewEnumerator0") (`self.HasLowHealthDefiner`)))
                    (:`then_1`
                      ;;[1 1 1] Has Shield
                      (`WorldState.AddWorldStateDefiner` _currentworldstate (enumliteral `/Game/Blueprints/EWorldState` "NewEnumerator2") (`self.HasShieldDefiner`)))
                    (:`then_2`
                      ;;[1 1 1] Has Weapon
                      (`WorldState.AddWorldStateDefiner` _currentworldstate (enumliteral `/Game/Blueprints/EWorldState` "NewEnumerator1") (`self.HasWeaponDefiner`)))
                    (:`then_3`
                      ;;[1 1 1] Is Enemy Dead
                      (`WorldState.AddWorldStateDefiner` _currentworldstate (enumliteral `/Game/Blueprints/EWorldState` "NewEnumerator4") (`self.IsEnemyDeadDefiner`)))
                    (:`then_4`
                      ;;[1 1 1] Is Enemy Visible
                      (`WorldState.AddWorldStateDefiner` _currentworldstate (enumliteral `/Game/Blueprints/EWorldState` "NewEnumerator3") (`self.IsEnemyVisibleDefiner`))
                      (`|ExecutionSequence`
                        (:`then_0`
                          ;[1 1 1] Creating Actions
                          ;;[1 1 1] Find Enemy
                          (`ActionTest.SetPrecondition` (`self.FindEnemyAction`) (enumliteral `/Game/Blueprints/EWorldState` "NewEnumerator3") false)
                          (`ActionTest.SetEffect` (`self.FindEnemyAction`) (enumliteral `/Game/Blueprints/EWorldState` "NewEnumerator3") true)
                          (`ActionTest.SetActionID` _findenemyaction 1)
                          (`KismetArrayLibrary.Array_Add` (`self.AllActions`) _findenemyaction))
                        (:`then_1`
                          ;;[1 1 1] Find Health
                          (`ActionTest.SetPrecondition` (`self.FindHealthAction`) _returnvalue_4 true)
                          (`ActionTest.SetEffect` (`self.FindHealthAction`) _returnvalue_4 false)
                          (`ActionTest.SetActionID` _findhealthaction 2)
                          (`KismetArrayLibrary.Array_Add` (`self.AllActions`) _findhealthaction))
                        (:`then_2`
                          ;;[1 1 1] Find Weapon
                          (`ActionTest.SetPrecondition` (`self.FindWeaponAction`) _returnvalue false)
                          (`ActionTest.SetEffect` (`self.FindWeaponAction`) _returnvalue true)
                          (`ActionTest.SetActionID` _findweaponaction 3)
                          (`KismetArrayLibrary.Array_Add` (`self.AllActions`) _findweaponaction))
                        (:`then_3`
                          ;;[1 1 1] Melee Action
                          (`ActionTest.SetPrecondition` (`self.MeleeAction`) (enumliteral `/Game/Blueprints/EWorldState` "NewEnumerator3") true)
                          (`ActionTest.SetPrecondition` (`self.MeleeAction`) _returnvalue_2 false)
                          (`ActionTest.SetEffect` (`self.MeleeAction`) _returnvalue_2 true)
                          (`ActionTest.SetActionID` _meleeaction 4)
                          (`KismetArrayLibrary.Array_Add` (`self.AllActions`) _meleeaction))
                        (:`then_4`
                          ;;[1 1 1] Shoot Action
                          (`ActionTest.SetPrecondition` (`self.ShootAction`) (enumliteral `/Game/Blueprints/EWorldState` "NewEnumerator4") false)
                          (`ActionTest.SetPrecondition` (`self.ShootAction`) (enumliteral `/Game/Blueprints/EWorldState` "NewEnumerator3") true)
                          (`ActionTest.SetPrecondition` (`self.ShootAction`) (enumliteral `/Game/Blueprints/EWorldState` "NewEnumerator1") true)
                          (`ActionTest.SetEffect` (`self.ShootAction`) (enumliteral `/Game/Blueprints/EWorldState` "NewEnumerator4") true)
                          (`ActionTest.SetEffect` (`self.ShootAction`) (enumliteral `/Game/Blueprints/EWorldState` "NewEnumerator1") false)
                          (`ActionTest.SetActionID` _shootaction 5)
                          (`KismetArrayLibrary.Array_Add` (`self.AllActions`) _shootaction))
                        (:`then_5`
                          ;;[1 1 1] Shield Action
                          (`ActionTest.SetPrecondition` (`self.ShieldAction`) _returnvalue_3 false)
                          (`ActionTest.SetEffect` (`self.ShieldAction`) _returnvalue_3 true)
                          (`ActionTest.SetActionID` _shieldaction 6)
                          (`KismetArrayLibrary.Array_Add` (`self.AllActions`) _shieldaction))))))))))))))