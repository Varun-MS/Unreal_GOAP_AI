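; BP_Action_FindShield is a GOAP action that has an AI agent search for a shield.
; Execute caches the GOAP AI controller, sets its status text, marks the action running and starts a looping FindShield timer.
; Each tick of that timer checks world state against the action's effect state, either sending the agent to a random waypoint or clearing the timer and completing the action.
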(event `FindShield`
  ;[1 1 1] Check WorldState against action effect state
  (if true
    (`AIController_Goap.GoToRandomWaypoint` (`self.controller`))
    (else
      (`KismetSystemLibrary.K2_ClearTimer` null "FindShield")
      (`self.SetActionStatus` "VE_Complete"))))

(event `self.Execute`
  (params (aiController :type "AIController Object Reference"))
  (bind _asbp_aicontroller_goap (cast `/Game/Blueprints/BP_AIController_Goap` aiController))
  (bind _output_get (set `self.controller` _asbp_aicontroller_goap))
  (`/Game/Blueprints/BP_AIController_Goap.SetAIStatus` _output_get "Looking For Shield")
  (`self.SetActionStatus` "VE_Running")
  (`KismetSystemLibrary.K2_SetTimer` null "FindShield" 5.0 true))