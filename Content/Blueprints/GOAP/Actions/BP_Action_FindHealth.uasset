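; GOAP action that sends an AI looking for health by wandering between random waypoints while its health is low.
; Execute caches the GOAP controller and world state manager, sets the AI status and action to running, then starts a looping FindHealth timer.
; Each tick of that timer polls the low-health world state, either requesting another random waypoint or clearing the timer and completing the action.
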(event `FindHealth`
  ;[1 1 1] Check if health is low
  (bind _returnvalue (`WorldState.GetWorldStateDefiner` (`WorldStateManager.CurrentWorldState` (`self.WorldStateManager`)) (enumliteral `/Game/Blueprints/EWorldState` "NewEnumerator0")))
  (if (`WorldStateDefiner.IsTrue` _returnvalue)
    (`AIController_Goap.GoToRandomWaypoint` (`self.controller`))
    (else
      (`KismetSystemLibrary.K2_ClearTimer` null "FindHealth")
      (`self.SetActionStatus` "VE_Complete"))))

(event `self.Execute`
  (params (AiController :type "AIController Object Reference") (WorldStateManager :type "WorldStateManager Object Reference"))
  (bind _asbp_ac_world_state_manager (cast `/Game/Blueprints/GOAP/WorldStateManager/BP_AC_WorldStateManager` WorldStateManager))
  (set `self.WorldStateManager` _asbp_ac_world_state_manager)
  (bind _asbp_aicontroller_goap (cast `/Game/Blueprints/BP_AIController_Goap` AiController))
  (bind _output_get (set `self.controller` _asbp_aicontroller_goap))
  (`/Game/Blueprints/BP_AIController_Goap.SetAIStatus` _output_get "Looking For Health")
  (`self.SetActionStatus` "VE_Running")
  (`KismetSystemLibrary.K2_SetTimer` null "FindHealth" 5.0 true))