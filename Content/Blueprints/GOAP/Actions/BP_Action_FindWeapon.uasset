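; GOAP action that has an AI agent wander in search of a weapon.
; Execute caches the GOAP AI controller and world state manager, sets the AI status text, marks the action running and starts a looping FindWeapon timer.
; Each tick of that timer checks the action's effect in the current world state, either clearing the timer and completing the action or sending the controller to a random waypoint.
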(event `FindWeapon`
  ;[1 1 1] Check WorldState against action effect state
  (bind _returnvalue (`WorldState.GetWorldStateDefiner` (`WorldStateManager.CurrentWorldState` (`self.WorldStateManager`)) (enumliteral `/Game/Blueprints/EWorldState` "NewEnumerator1")))
  (if (`WorldStateDefiner.IsTrue` _returnvalue)
    (`KismetSystemLibrary.K2_ClearTimer` null "FindWeapon")
    (`self.SetActionStatus` "VE_Complete")
    (else
      (`AIController_Goap.GoToRandomWaypoint` (`self.controller`)))))

(event `self.Execute`
  (params (AiController :type "AIController Object Reference") (WorldStateManager :type "WorldStateManager Object Reference"))
  (bind _asbp_ac_world_state_manager (cast `/Game/Blueprints/GOAP/WorldStateManager/BP_AC_WorldStateManager` WorldStateManager)
    (:`then`
      (set `self.WorldStateManager` _asbp_ac_world_state_manager)
      (bind _asbp_aicontroller_goap (cast `/Game/Blueprints/BP_AIController_Goap` AiController))
      (bind _output_get (set `self.controller` _asbp_aicontroller_goap))
      (`/Game/Blueprints/BP_AIController_Goap.SetAIStatus` _output_get "Looking For Weapon")
      (`self.SetActionStatus` "VE_Running")
      (`KismetSystemLibrary.K2_SetTimer` null "FindWeapon" 5.0 true))
    (:`CastFailed`
      (`KismetSystemLibrary.PrintString` null "Cast Failed"))))