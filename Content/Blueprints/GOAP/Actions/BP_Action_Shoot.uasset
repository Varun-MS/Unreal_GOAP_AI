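; GOAP action that makes an AI agent shoot at its enemy.
; Execute caches the world state manager, controller and enemy, then starts looping timers for firing and for aiming the controller's focal point at the enemy.
; Each shot applies fixed damage only while three world-state flags hold the required values.
; Otherwise, it clears both timers and marks the action complete.
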(event `LookAtEnemy`
  ;[1 1 1] Update enemy location
  (bind _output_get (set `self.EnemyLocation` (`Actor.K2_GetActorLocation` (`self.EnemyRef`))))
  (`AIController.K2_SetFocalPoint` (`self.Controller`) _output_get))

(event `Shoot`
  (bind _currentworldstate (`WorldStateManager.CurrentWorldState` (`self.WorldStateManager`)))
  ;[1 1 1] Check WorldState against action effect state
  (bind _returnvalue (`WorldState.GetWorldStateDefiner` _currentworldstate (enumliteral `/Game/Blueprints/EWorldState` "NewEnumerator1")))
  (bind _returnvalue_2 (`WorldState.GetWorldStateDefiner` _currentworldstate (enumliteral `/Game/Blueprints/EWorldState` "NewEnumerator3")))
  (bind _returnvalue_3 (`WorldState.GetWorldStateDefiner` _currentworldstate (enumliteral `/Game/Blueprints/EWorldState` "NewEnumerator4")))
  (if (and (and _returnvalue _returnvalue_2) (not _returnvalue_3))
    ;[1 1 1] Do Damage to enemy health
    (`/Game/Blueprints/BP_AI_CHaracter.DoDamage` (`self.EnemyRef`) 15.0)
    (else
      (`KismetSystemLibrary.K2_ClearTimer` null "Shoot")
      (`KismetSystemLibrary.K2_ClearTimer` null "LookAtEnemy")
      (`self.SetActionStatus` "VE_Complete"))))

(event `self.Execute`
  (params (AiController :type "AIController Object Reference") (WorldStateManager :type "WorldStateManager Object Reference"))
  (bind _asbp_ac_world_state_manager (cast `/Game/Blueprints/GOAP/WorldStateManager/BP_AC_WorldStateManager` WorldStateManager))
  (set `self.WorldStateManager` _asbp_ac_world_state_manager)
  (bind _asbp_aicontroller_goap (cast `/Game/Blueprints/BP_AIController_Goap` AiController))
  (bind _output_get (set `self.Controller` _asbp_aicontroller_goap))
  (bind _asbp_ai_character (cast `/Game/Blueprints/BP_AI_CHaracter` (`Actor.GetOwner` (`self.Controller`))))
  (set `self.EnemyRef` (`/Game/Blueprints/BP_AI_CHaracter.EnemyRef` _asbp_ai_character))
  (`/Game/Blueprints/BP_AIController_Goap.SetAIStatus` _output_get "Shooting!")
  (`self.SetActionStatus` "VE_Running")
  (`KismetSystemLibrary.K2_SetTimer` null "Shoot" 2.0 true)
  (`KismetSystemLibrary.K2_SetTimer` null "LookAtEnemy" 0.1 true))